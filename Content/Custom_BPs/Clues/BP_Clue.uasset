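; BP_Clue is a world clue actor that shows a ClueWidget marker when the first-person player comes near.
; The widget starts transparent, and each tick compares the player's distance to MinDistToDraw.
; A timeline lerps its color alpha, playing forward in range and reversing out of range.
; While the player's CanCheckItem flag is true, the widget is set fully transparent instead.
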(event EventTick
  (params (DeltaSeconds :type Float%20%28single-precision%29))
  (bind _closeenough (CallFunction|IsPlayercloseEnough (Transformation|GetActorLocation) (Transformation|GetActorLocation (Game|Player|GetPlayerPawn 0)) (Variables|Default|GetminDistToDraw)))
  (if (Variables|/Game/FP_Controller/BP_FP_Character.BP_FP_Character_C|GetcanCheckItem (Variables|Default|Getplayer))
    (Appearance|SetColorandOpacity (.AsClue%20Widget (Utilities|Casting|CastToClueWidget (UserInterface|GetWidget (Variables|Default|GetWidget)))) "(R=1.000000,G=1.000000,B=1.000000,A=0.000000)" :!class /Script/UMG.UserWidget)
    (elif _closeenough
      (bind _newtrack_0 (Timeline|Timeline_0 Play)
        (:Update
          (Appearance|SetColorandOpacity (.AsClue%20Widget (Utilities|Casting|CastToClueWidget (UserInterface|GetWidget (Variables|Default|GetWidget)))) (Math|Color|Lerp(LinearColor) "(R=1.000000,G=1.000000,B=1.000000,A=0.000000)" "(R=1.000000,G=1.000000,B=1.000000,A=1.000000)" _newtrack_0) :!class /Script/UMG.UserWidget)))
      (else
        (Timeline|Timeline_0 Reverse)))))

(event EventBeginPlay
  (Appearance|SetColorandOpacity (.AsClue%20Widget (Utilities|Casting|CastToClueWidget (UserInterface|GetWidget (Variables|Default|GetWidget)))) "(R=1.000000,G=1.000000,B=1.000000,A=0.000000)" :!class /Script/UMG.UserWidget)
  (Variables|Default|Setplayer (.AsBP%20FP%20Character (Utilities|Casting|CastToBP_FP_Character (Game|Player|GetPlayerPawn 0)))))

(fn ConstructionScript)

(fn IsPlayercloseEnough
  (params (V1 :type Vector) (V2 :type Vector) (InputPin :type Float%20%28double-precision%29))
  (return (<= (Math|Vector|Distance(Vector) V1 V2) InputPin)))